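; Arcade character Blueprint that spawns Level1Merge actors, apparently as pieces for a merge game.
; On BeginPlay it spawns the first piece at a fixed world location, starts its movement through CallMerge1Movement, then binds SpawnLevel1_Event to the SpawnLevel1 dispatcher.
; Each firing of that event increments Merge1Uses and spawns another moving piece at the same spot.
; A debug print of the counter is left unconnected.
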(event `self.ReceiveBeginPlay`
  (`|ExecutionSequence`
    (:`then_0`
      (bind _returnvalue (`|SpawnActorFromClass` "/Game/FinalBlueprints/Level1Merge.Level1Merge_C" (`KismetMathLibrary.MakeTransform` (585.0 80.0 1500.0)) "Undefined" "MultiplyWithRoot" null null))
      (`/Game/FinalBlueprints/Level1Merge.Merge1Movement` _returnvalue))
    (:`then_1`
      (add `self.SpawnLevel1` (delegate `SpawnLevel1_Event`)))))

(event `SpawnLevel1_Event`
  (set `self.Merge1Uses` (+ (`self.Merge1Uses`) 1))
  (bind _returnvalue (`|SpawnActorFromClass` "/Game/FinalBlueprints/Level1Merge.Level1Merge_C" (`KismetMathLibrary.MakeTransform` (585.0 80.0 1500.0)) "Undefined" "MultiplyWithRoot" null null))
  (`/Game/FinalBlueprints/Level1Merge.Merge1Movement` _returnvalue))

(fn `UserConstructionScript`)